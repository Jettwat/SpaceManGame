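; Moving platform Blueprint that travels along an array of waypoint actors, with configurable mesh, material, rate and optional looping.
; BeginPlay hides the waypoints and calls PlatformStart inside that loop, which resets to the first pair and plays MotionTimeline.
; The timeline lerps location between current and next waypoint positions, with an event that advances indices or restarts the path.
; Stop halts the timeline, while Start is an empty stub.
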(event Custom|Platform%20Start
  (bind _motiontimeline (Variables|Default|GetMotionTimeline))
  (CallFunction|SetFirstWaypoint)
  (Components|Timeline|SetPlayRate _motiontimeline (Variables|Default|GetRate))
  (Components|Timeline|PlayfromStart _motiontimeline))

(event EventBeginPlay
  (for _array_element (Variables|Default|GetWaypoints)
    (Rendering|SetActorHiddenInGame _array_element true)
    (CallFunction|PlatformStart)))

(fn ConstructionScript
  (bind _platform_mesh (Variables|Default|GetPlatform%20Mesh))
  (Components|StaticMesh|SetStaticMesh _platform_mesh (Variables|Default|GetStatic%20Mesh))
  (Rendering|Material|SetMaterial _platform_mesh 0 (Variables|Default|GetMaterial)))

(fn SetPositions
  (bind _waypoints (Variables|Default|GetWaypoints))
  (Variables|Default|SetCurrent%20Waypoint%20Position (Transformation|GetActorLocation (Utilities|Array|Get(acopy) _waypoints (Variables|Default|GetCurrent%20Waypoint%20Index))))
  (Variables|Default|SetNext%20Waypoint%20Position (Transformation|GetActorLocation (Utilities|Array|Get(acopy) _waypoints (Variables|Default|GetNext%20Waypoint%20Index)))))

(fn SetFirstWaypoint
  (Variables|Default|SetCurrent%20Waypoint%20Index 0)
  (Variables|Default|SetNext%20Waypoint%20Index 1)
  (CallFunction|SetPositions))

(fn SetNextWaypoint
  (bind _result (Math|Integer|IncrementInt (Variables|Default|GetCurrent%20Waypoint%20Index))
    (:%20%20
      (Variables|Default|SetCurrent%20Waypoint%20Index (+ _result 1))
      (CallFunction|SetPositions))))

(fn PathIsFinished
  (return (== (Variables|Default|GetNext%20Waypoint%20Index) (- (Utilities|Array|Length (Variables|Default|GetWaypoints)) 1))))

(fn Start)

(fn Stop
  (Audio|Components|Audio|Stop (Variables|Default|GetMotionTimeline)))