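; BP_Checkpoint is a checkpoint actor that sets the player's respawn point when something overlaps it.
; On begin overlap it recolors the floor and door, swaps the door mesh, shows its text and writes the RespawnLocation component's world position to the game manager's Respawn.
; Leaving the box restores the unclaimed material and hides the text, while the door mesh and saved respawn point remain.
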(event OnComponentEndOverlap(Box)
  (params (OverlappedComponent :type Primitive%20Component%20Object%20Reference) (OtherActor :type Actor%20Object%20Reference) (OtherComp :type Primitive%20Component%20Object%20Reference) (OtherBodyIndex :type Integer))
  (Rendering|Material|SetMaterial (Variables|Default|GetFloor) 0 "/Game/__MyContent/Materials/M_UnclaimedBlock.M_UnclaimedBlock")
  (Rendering|SetVisibility (Variables|Default|GetTextRender) false false))

(event Collision|EventActorBeginOverlap
  (params (OtherActor :type Actor%20Object%20Reference))
  (Rendering|Material|SetMaterial (Variables|Default|GetFloor) 0 "/Engine/MapTemplates/Materials/BasicAsset01.BasicAsset01")
  (Components|StaticMesh|SetStaticMesh (Variables|Default|GetDoor) "/Game/StarterContent/Architecture/Wall_Door_400x300.Wall_Door_400x300")
  (Rendering|SetVisibility (Variables|Default|GetTextRender) true false)
  (bind _my_game_manager (CallFunction|GetMyGameManager))
  (Variables|/Game/__MyContent/Blueprints/BP_MyGameManager.BP_MyGameManager_C|SetRespawn _my_game_manager (Transformation|GetWorldLocation (Variables|Default|GetRespawn%20Location))))

(fn ConstructionScript)